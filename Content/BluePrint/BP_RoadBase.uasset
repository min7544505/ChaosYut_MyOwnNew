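; BP_RoadBase is a board-game road node linking to next and previous roads and tracking the pieces on it.
; GetNextRoad returns the sole link or, at a fork, picks the outer or diagonal road from PreferDiagonal, with debug prints.
; GetPrevRoad handles zero or one link; its fork branch is unconnected.
; Enter and exit functions update OccupyingPieces and each piece's CurrentRoad, while clicking prints RoadID.
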(event `self.ReceiveActorOnClicked`
  (params (ButtonPressed :type "Key Structure"))
  (`KismetSystemLibrary.PrintString` (`KismetStringLibrary.Conv_NameToString` (`self.RoadID`))))

(fn `GetNextRoad`
  (params (bPreferDiagonal :type Boolean))
  (returns (NextRoad :type "/Game/BluePrint/BP_RoadBase Object Reference"))
  (bind _returnvalue (`KismetArrayLibrary.Array_Length` (`self.NextRoads`)))
  (`KismetSystemLibrary.PrintString` (`KismetStringLibrary.Conv_IntToString` _returnvalue) true true (struct :`R` 1.0 :`G` 0.003177 :`B` 0.967035 :`A` 1.0) 10.0)
  (switch `int` _returnvalue
    (:`0`
      ; 앞에 길이 없을 때 (결승점)
      (return null))
    (:`1`
      ; 앞에 길이 1개 일 때 (일반길)
      (return (`|GetArrayItem` (`self.NextRoads`))))
    (:`2`
      (`KismetSystemLibrary.PrintString` "일단 2개는 맞아" true true (struct :`R` 0.241589 :`G` 1.0 :`B` 0.399105 :`A` 1.0) 10.0)
      (if bPreferDiagonal
        (`KismetSystemLibrary.PrintString` "트루로 반환" true true (struct :`R` 0.241589 :`G` 1.0 :`B` 0.399105 :`A` 1.0) 10.0)
        ; 길 2개 중 대각선
        (return (`|GetArrayItem` (`self.NextRoads`) 1))
        (else
          (`KismetSystemLibrary.PrintString` "펄스로 반환" true true (struct :`R` 0.241589 :`G` 1.0 :`B` 0.399105 :`A` 1.0) 10.0)
          ; 길 2개 중 외곽
          (return (`|GetArrayItem` (`self.NextRoads`))))))))

(fn `GetPrevRoad`
  (params (bPreferDiagonal :type Boolean))
  (returns (PrevRoad :type "/Game/BluePrint/BP_RoadBase Object Reference"))
  (switch `int` (`KismetArrayLibrary.Array_Length` (`self.PrevRoads`))
    (:`0`
      ; 뒷 길 X (시작점)
      (return null))
    (:`1`
      ; 뒷 길 1 개 (일반)
      (return (`|GetArrayItem` (`self.PrevRoads`))))))

(fn `OnPieceEnter`
  (params (Piece :type "/Game/BluePrint/BP_YutPiece Object Reference"))
  (set `/Game/BluePrint/BP_YutPiece.CurrentRoad` self Piece)
  (`KismetArrayLibrary.Array_Add` (`self.OccupyingPieces`) Piece))

(fn `OnPieceExit`
  (params (Piece :type "/Game/BluePrint/BP_YutPiece Object Reference"))
  (`KismetArrayLibrary.Array_RemoveItem` (`self.OccupyingPieces`) Piece)
  (set `/Game/BluePrint/BP_YutPiece.CurrentRoad` null Piece))

(fn `UserConstructionScript`)