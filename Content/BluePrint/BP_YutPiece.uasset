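; Board piece for a Yut game that moves along BP_YutRoad paths, stacks with teammates and can return to its waiting position.
; BeginPlay automatically requests a ten-step path from BP_YutBoard and teleports through it via MoveThrough.
; MoveTo lands on the last road, marking a finish, merging same-team pieces under one carrier, or resetting itself upon meeting an uncarried opponent.
; Resets cascade to stacked pieces; clicking only prints debug text.
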(event `self.ReceiveBeginPlay`
  (set `self.WatingPosition` (`self.K2_GetActorLocation`))
  (`KismetSystemLibrary.Delay` 1.0)
  (bind _outactors (`GameplayStatics.GetAllActorsOfClass` "/Game/BluePrint/BP_YutBoard.BP_YutBoard_C"))
  (bind _asbp_yut_board (cast `/Game/BluePrint/BP_YutBoard` (`|GetArrayItem` _outactors)))
  (bind _path (`/Game/BluePrint/BP_YutBoard.CalculatePath` _asbp_yut_board (`/Game/BluePrint/BP_YutBoard.StartRoad` _asbp_yut_board) 10 false))
  (`self.MoveAlongPath` _path))

(event `self.Box.OnClicked`
  (params (TouchedComponent :type "PrimitiveComponent Object Reference") (ButtonPressed :type "Key Structure"))
  (`KismetSystemLibrary.PrintString` "개당"))

(event `MoveAlongPath`
  (params (Path :type "Array of /Game/BluePrint/BP_RoadBase Object Reference"))
  (bind _returnvalue (`KismetArrayLibrary.Array_Length` Path))
  (bind _returnvalue_2 (- _returnvalue 1))
  (if (> _returnvalue 0)
    (for _index (range (+ _returnvalue_2 1))
      (if (== _index _returnvalue_2)
        (bind _output (`|GetArrayItem` Path _index))
        (`self.MoveTo` _output)
        (else
          (`self.MoveThrough` _output)
          (`KismetSystemLibrary.Delay` 1.0))))))

(fn `MoveThrough`
  (params (TargetRoad :type "/Game/BluePrint/BP_RoadBase Object Reference"))
  (`/Engine/EditorBlueprintResources/StandardMacros.IsValid` TargetRoad
    (:`Is Valid`
      (`self.K2_SetActorLocation` (`self.K2_GetActorLocation` TargetRoad))
      (return))
    (:`Is Not Valid`
      (return))))

(fn `MoveTo`
  (params (TargetRoad :type "/Game/BluePrint/BP_RoadBase Object Reference"))
  (`/Engine/EditorBlueprintResources/StandardMacros.IsValid` TargetRoad
    (:`Is Valid`
      (`/Engine/EditorBlueprintResources/StandardMacros.IsValid` (`self.CurrentRoad`)
        (:`Is Valid`
          (if true
            (`/Game/BluePrint/BP_RoadBase.OnPieceExit` (`self.CurrentRoad`) self)))
        (:`Is Not Valid`
          _))
      (`self.K2_SetActorLocation` (`self.K2_GetActorLocation` TargetRoad))
      (`/Game/BluePrint/BP_RoadBase.OnPieceEnter` TargetRoad self)
      (if (== (`KismetArrayLibrary.Array_Length` (`/Game/BluePrint/BP_RoadBase.NextRoads` TargetRoad)) 0)
        (set `self.IsFinished` true)
        (return)
        (else
          (for _array_element (`/Game/BluePrint/BP_RoadBase.OccupyingPieces` TargetRoad)
            (if (== _array_element self)
              _
              (elif (== (`/Game/BluePrint/BP_YutPiece.TeamIndex` _array_element) (`self.TeamIndex`))
                (`self.StackWith` _array_element)
                (else
                  (`/Engine/EditorBlueprintResources/StandardMacros.IsValid` (`/Game/BluePrint/BP_YutPiece.CarrierPiece` _array_element)
                    (:`Is Not Valid`
                      (`self.ResetToWating`))))))))))
    (:`Is Not Valid`
      (return))))

(fn `ResetToWating`
  (`/Engine/EditorBlueprintResources/StandardMacros.IsValid` (`self.CurrentRoad`)
    (:`Is Valid`
      (`/Game/BluePrint/BP_RoadBase.OnPieceExit` (`self.CurrentRoad`) self))
    (:`Is Not Valid`
      _))
  (set `self.CurrentRoad` null)
  (set `self.CarrierPiece` null)
  (for _array_element (`self.StackedPieces`)
    (`self.ResetToWating` _array_element))
  (`KismetArrayLibrary.Array_Clear` (`self.StackedPieces`))
  (`self.K2_SetActorLocation` (`self.WatingPosition`)))

(fn `StackWith`
  (params (OtherPiece :type "/Game/BluePrint/BP_YutPiece Object Reference"))
  (locals (BottomPiece :type "/Game/BluePrint/BP_YutPiece Object Reference"))
  (`/Engine/EditorBlueprintResources/StandardMacros.IsValid` (`/Game/BluePrint/BP_YutPiece.CarrierPiece` OtherPiece)
    (:`Is Valid`
      (set `local.BottomPiece` (`/Game/BluePrint/BP_YutPiece.CarrierPiece` OtherPiece)))
    (:`Is Not Valid`
      (set `local.BottomPiece` OtherPiece)))
  (for _array_element (`self.StackedPieces`)
    (set `/Game/BluePrint/BP_YutPiece.CarrierPiece` (`local.BottomPiece`) _array_element)
    (`KismetArrayLibrary.Array_Add` (`/Game/BluePrint/BP_YutPiece.StackedPieces` (`local.BottomPiece`)) _array_element))
  (`KismetArrayLibrary.Array_Clear` (`self.StackedPieces`))
  (`KismetArrayLibrary.Array_Add` (`/Game/BluePrint/BP_YutPiece.StackedPieces` (`local.BottomPiece`)) self)
  (set `self.CarrierPiece` (`local.BottomPiece`))
  (set `self.CurrentRoad` null))

(fn `UserConstructionScript`)