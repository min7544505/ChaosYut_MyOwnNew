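; Yut board actor that builds the game's network of road spaces from the DT_BoardLayout data table at BeginPlay.
; InitializeBoard spawns a road subclass per row type (normal, branch, merge, center) into the AllRoads map and records START.
; A second pass, SetupConnections, links next and previous roads from pipe-delimited IDs.
; CalculatePath steps through GetNextRoad with a diagonal preference; GetRoadByID is an empty stub, and BeginPlay debug-prints C2's links.
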(event `self.ReceiveBeginPlay`
  (`self.InitializeBoard`)
  (`self.DebugPrintConnectionRoads` "C2"))

(fn `CalculatePath`
  (params (StartRoad :type "/Game/BluePrint/BP_RoadBase Object Reference") (Steps :type Integer) (bPreferDiagonal :type Boolean))
  (returns (Path :type "Array of /Game/BluePrint/BP_RoadBase Object Reference"))
  (locals (CurrentRoad :type "/Game/BluePrint/BP_RoadBase Object Reference") (LoopIndex :type Integer) (PathArray :type "Array of /Game/BluePrint/BP_RoadBase Object Reference"))
  (set `local.CurrentRoad` StartRoad)
  (for _ (range Steps)
    (bind _nextroad (`/Game/BluePrint/BP_RoadBase.GetNextRoad` (`local.CurrentRoad`) bPreferDiagonal))
    (`/Engine/EditorBlueprintResources/StandardMacros.IsValid` _nextroad
      (:`Is Valid`
        _)
      (:`Is Not Valid`
        _))
    (`KismetArrayLibrary.Array_Add` (`local.PathArray`) _nextroad)
    (set `local.CurrentRoad` _nextroad))
  (return (`local.PathArray`)))

(fn `DebugPrintConnectionRoads`
  (params (Key :type "Name (by ref)"))
  (bind (_value _returnvalue) (`BlueprintMapLibrary.Map_Find` (`self.AllRoads`) Key))
  ; Key 값에다가 DataTable 에 있는 자리 이름 넣으면,  find Next and Prev Roads
  (`/Engine/EditorBlueprintResources/StandardMacros.IsValid` _value
    (:`Is Valid`
      (if _returnvalue
        (for _array_element (`/Game/BluePrint/BP_RoadBase.NextRoads` _value)
          (`KismetSystemLibrary.PrintString` (`KismetStringLibrary.Concat_StrStr` "\"C1 NextRoad: \"" (`KismetStringLibrary.Conv_NameToString` (`/Game/BluePrint/BP_RoadBase.RoadID` _array_element)))) ; Next is blue
        )
        (for _array_element_2 (`/Game/BluePrint/BP_RoadBase.PrevRoads` _value)
          (`KismetSystemLibrary.PrintString` (`KismetStringLibrary.Concat_StrStr` "\"C1 PrevRoad: \"" (`KismetStringLibrary.Conv_NameToString` (`/Game/BluePrint/BP_RoadBase.RoadID` _array_element_2))) true true (struct :`R` 0.894713 :`G` 1.0 :`B` 0.112682 :`A` 1.0)) ; Prev is Yellow
        )))))

(fn `GetRoadByID`
  (params (ID :type Name))
  (returns (BP_RoadBase :type "/Game/BluePrint/BP_RoadBase Object Reference"))
  (return null))

(fn `InitializeBoard`
  (bind _outrownames (`DataTableFunctionLibrary.GetDataTableRowNames` (`self.BoardLayoutTable`)))
  (for _array_element _outrownames
    (bind _returnvalue (`|GetDataTableRow` "/Game/Data/DT_BoardLayout.DT_BoardLayout" _array_element)
      (:`then`
        (bind _spawnroad (`self.SpawnRoadByType` _returnvalue))
        (`BlueprintMapLibrary.Map_Add` (`self.AllRoads`) (`.RoadID_6_D9A65EE548E5213130AC3495B9B49455` (break `/Game/Data/ST_RoadData` _returnvalue)) _spawnroad))))
  (set `self.StartRoad` (`BlueprintMapLibrary.Map_Find` (`self.AllRoads`) "START"))
  (`self.SetupConnections`))

(fn `SetupConnections`
  (locals (CurrentRoad :type "/Game/BluePrint/BP_RoadBase Object Reference"))
  (bind _outrownames (`DataTableFunctionLibrary.GetDataTableRowNames` "/Game/Data/DT_BoardLayout.DT_BoardLayout"))
  (for _array_element _outrownames
    (bind _returnvalue (`|GetDataTableRow` "/Game/Data/DT_BoardLayout.DT_BoardLayout" _array_element)
      (:`then`
        (bind ((`RoadID_6_D9A65EE548E5213130AC3495B9B49455` _roadid) (`NextRoads_19_333E0AC34C0244BE7BE968A4EFAC8E29` _nextroads) (`PrevRoads_21_626938184E8D1A2E0B9018B52F89849C` _prevroads)) (break `/Game/Data/ST_RoadData` _returnvalue))
        (set `local.CurrentRoad` (`BlueprintMapLibrary.Map_Find` (`self.AllRoads`) _roadid))
        (bind _returnvalue_2 (`KismetStringLibrary.ParseIntoArray` _nextroads "|"))
        (for _array_element_2 _returnvalue_2
          (`KismetArrayLibrary.Array_Add` (`/Game/BluePrint/BP_RoadBase.NextRoads` (`local.CurrentRoad`)) (`BlueprintMapLibrary.Map_Find` (`self.AllRoads`) (`KismetStringLibrary.Conv_StringToName` _array_element_2))))
        (bind _returnvalue_3 (`KismetStringLibrary.ParseIntoArray` _prevroads "|"))
        (for _array_element_3 _returnvalue_3
          (`KismetArrayLibrary.Array_Add` (`/Game/BluePrint/BP_RoadBase.PrevRoads` (`local.CurrentRoad`)) (`BlueprintMapLibrary.Map_Find` (`self.AllRoads`) (`KismetStringLibrary.Conv_StringToName` _array_element_3)))))))
  (return))

(fn `SpawnRoadByType`
  (params (RoadData :type "/Game/Data/ST_RoadData Structure"))
  (returns (SpawnRoad :type "/Game/BluePrint/BP_RoadBase Object Reference"))
  (locals (SpawnedRoad :type "/Game/BluePrint/BP_RoadBase Object Reference"))
  (bind ((`RoadType_8_2898C69E4C52DFDE7562ED8F2598149C` _roadtype) (`PositionX_10_E502DAA04B3F62163873138AE3462D1C` _positionx) (`PositionY_12_77F04023466C3A8D71F457A0953D4BE6` _positiony) (`PositionZ_26_AA480D5B46C3EF451B81109680800BFC` _positionz)) (break `/Game/Data/ST_RoadData` RoadData))
  (bind ((`RoadID_6_D9A65EE548E5213130AC3495B9B49455` _roadid) (`RoadType_8_2898C69E4C52DFDE7562ED8F2598149C` _roadtype_2) (`IsCorner_23_BA45159440B61CD3F16895958A284414` _iscorner) (`IsDiagonal_25_C5B03AD34D4D11C4113E8594BD2AAEF6` _isdiagonal)) (break `/Game/Data/ST_RoadData` RoadData))
  (bind _returnvalue (`KismetMathLibrary.MakeTransform` (`KismetMathLibrary.MakeVector` _positionx _positiony _positionz)))
  (switch `/Game/Data/E_RoadType` _roadtype
    (:`NewEnumerator0`
      (bind _returnvalue_2 (`|SpawnActorFromClass` "/Game/BluePrint/BP_RoadBase.BP_RoadBase_C" _returnvalue "Undefined" "MultiplyWithRoot" null null))
      (set `local.SpawnedRoad` _returnvalue_2))
    (:`NewEnumerator1`
      (bind _returnvalue_3 (`|SpawnActorFromClass` "/Game/BluePrint/BP_BranchRoad.BP_BranchRoad_C" _returnvalue "Undefined" "MultiplyWithRoot" null null))
      (set `local.SpawnedRoad` _returnvalue_3))
    (:`NewEnumerator2`
      (bind _returnvalue_4 (`|SpawnActorFromClass` "/Game/BluePrint/BP_MergedRoad.BP_MergedRoad_C" _returnvalue "Undefined" "MultiplyWithRoot" null null))
      (set `local.SpawnedRoad` _returnvalue_4))
    (:`NewEnumerator3`
      (bind _returnvalue_5 (`|SpawnActorFromClass` "/Game/BluePrint/BP_CenterRoad.BP_CenterRoad_C" _returnvalue "Undefined" "MultiplyWithRoot" null null))
      (set `local.SpawnedRoad` _returnvalue_5)))
  (set `/Game/BluePrint/BP_RoadBase.RoadID` _roadid (`local.SpawnedRoad`))
  (set `/Game/BluePrint/BP_RoadBase.RoadType` _roadtype_2 (`local.SpawnedRoad`))
  (set `/Game/BluePrint/BP_RoadBase.IsCorner` _iscorner (`local.SpawnedRoad`))
  (set `/Game/BluePrint/BP_RoadBase.IsDiagonal` _isdiagonal (`local.SpawnedRoad`))
  (return (`local.SpawnedRoad`)))

(fn `UserConstructionScript`)